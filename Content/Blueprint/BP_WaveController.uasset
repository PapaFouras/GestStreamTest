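; Actor that animates a row of instanced static meshes in a traveling vertical wave.
; The construction script lays NbInstances along the actor's right vector as HISM instances.
; Each Tick, UpdateHISMLocations accumulates world time, offsets it by each instance's index ratio, wraps it, and samples WaveCurve, scaled by WaveHeight, for height along the up vector.
; An older Timeline-driven version remains in the EventGraph but never runs.
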(event `self.ReceiveBeginPlay`)

(event `self.ReceiveTick`
  (params (DeltaSeconds :type "Float (single-precision)"))
  (`self.UpdateHISMLocations`))

(fn `UpdateHISMLocations`
  (locals (CurrentIndex :type Integer))
  (bind (_returnvalue_location _returnvalue_rotation) (`KismetMathLibrary.BreakTransform` (`self.GetTransform`)))
  (set `self.TimeSinceBeginning` (+ (`self.TimeSinceBeginning`) (`GameplayStatics.GetWorldDeltaSeconds`)))
  (for _index (range (+ (`self.nbInstances`) 1))
    (set `local.CurrentIndex` _index)
    (`InstancedStaticMeshComponent.UpdateInstanceTransform` (`self.HierarchicalInstancedStaticMesh`) (`local.CurrentIndex`) (`KismetMathLibrary.MakeTransform` (+ _returnvalue_location (* (* _index 150) (`self.GetActorRightVector`)) (* (`self.GetActorUpVector`) (* (`CurveFloat.GetFloatValue` (`self.WaveCurve`) (mod (+ (`self.TimeSinceBeginning`) (/ (`local.CurrentIndex`) (`self.nbInstances`))) 1.0)) (`self.WaveHeight`)))) _returnvalue_rotation) true false false)))

(fn `UserConstructionScript`
  (bind (_returnvalue_location _returnvalue_rotation) (`KismetMathLibrary.BreakTransform` (`self.GetTransform`)))
  (for _index (range (+ (`self.nbInstances`) 1))
    (`InstancedStaticMeshComponent.AddInstance` (`self.HierarchicalInstancedStaticMesh`) (`KismetMathLibrary.MakeTransform` (+ _returnvalue_location (* (* _index 150) (`self.GetActorRightVector`))) _returnvalue_rotation) true)))