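; Test actor for Game Feature plugins and modular components, toggling its own registration as a component receiver at runtime.
; On BeginPlay it loads MyGameFeature2 by console command and enables input from the first player controller.
; The O key flip-flops between removing and adding it as a GameFrameworkComponentManager receiver, starting with removal.
; EndPlay deactivates the plugin by console command.
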(event `self.ReceiveBeginPlay`
  (`KismetSystemLibrary.ExecuteConsoleCommand` "LoadGameFeaturePlugin  MyGameFeature2" null)
  (`self.EnableInput` (`GameplayStatics.GetPlayerController` 0)))

(event `Key|O`
  (params (Key :type "Key Structure"))
  (:`Pressed`
    (`/Engine/EditorBlueprintResources/StandardMacros.FlipFlop`
      (:`A`
        (`GameFrameworkComponentManager.RemoveReceiver` (subsystem `GameFrameworkComponentManager`) self))
      (:`B`
        (`GameFrameworkComponentManager.AddReceiver` (subsystem `GameFrameworkComponentManager`) self true)))))

(event `self.ReceiveEndPlay`
  (params (EndPlayReason :type "EEndPlayReason Enum" :default "Destroyed"))
  (`KismetSystemLibrary.ExecuteConsoleCommand` "DeactivateGameFeaturePlugin  MyGameFeature2" null))

(fn `UserConstructionScript`)